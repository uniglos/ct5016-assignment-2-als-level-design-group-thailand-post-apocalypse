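; Timed door actor that destroys itself 15 seconds after the player interacts with it.
; Its trigger box enables input and shows an "E - Open Door" prompt on BP_Player, clearing both when the overlap ends.
; Interact sets an Opening flag, which Tick polls to run the delay and destroy the actor; leaving the trigger does not cancel the countdown.
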(event OnComponentBeginOverlap(TriggerBox)
  (params (OverlappedComponent :type Primitive%20Component%20Object%20Reference) (OtherActor :type Actor%20Object%20Reference) (OtherComp :type Primitive%20Component%20Object%20Reference) (OtherBodyIndex :type Integer) (bFromSweep :type Boolean) (SweepResult :type Hit%20Result%20Structure%20%28by%20ref%29))
  (bind _asbp_player (Utilities|Casting|CastToBP_Player OtherActor))
  (Input|EnableInput (Game|GetPlayerController 0))
  (Variables|/Game/Blueprints/BP_Player.BP_Player_C|SetCurrentInteractText _asbp_player "E - Open Door"))

(event OnComponentEndOverlap(TriggerBox)
  (params (OverlappedComponent :type Primitive%20Component%20Object%20Reference) (OtherActor :type Actor%20Object%20Reference) (OtherComp :type Primitive%20Component%20Object%20Reference) (OtherBodyIndex :type Integer))
  (bind _asbp_player (Utilities|Casting|CastToBP_Player OtherActor))
  (Input|DisableInput (Game|GetPlayerController 0))
  (Variables|/Game/Blueprints/BP_Player.BP_Player_C|SetCurrentInteractText _asbp_player ""))

(event EventBeginPlay
  (Variables|Actor|SetbCanBeDamaged true)
  (Variables|Default|Setopening false))

(event Collision|EventActorBeginOverlap
  (params (OtherActor :type Actor%20Object%20Reference)))

(event EventTick
  (params (DeltaSeconds :type Float%20%28single-precision%29))
  (if (Variables|Default|Getopening)
    (Utilities|FlowControl|Delay 15.0)
    (Actor|DestroyActor)))

(event Input|ActionEvents|InputActionInteract
  (params (Key :type Key%20Structure :default "None"))
  (:Pressed
    (Variables|Default|Setopening true)))

(fn ConstructionScript)