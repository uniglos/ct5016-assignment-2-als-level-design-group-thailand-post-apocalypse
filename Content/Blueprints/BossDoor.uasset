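; BossDoor is a locked door actor that disappears once the level's key unlocks it.
; On BeginPlay it finds the KeyScript actor, then polls its DoorsOpen flag every Tick and destroys itself when the flag is set.
; A Trigger component sets the player's interact text to "Locked" on overlap and clears it when the player leaves.
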(event OnComponentBeginOverlap(Trigger)
  (params (OverlappedComponent :type Primitive%20Component%20Object%20Reference) (OtherActor :type Actor%20Object%20Reference) (OtherComp :type Primitive%20Component%20Object%20Reference) (OtherBodyIndex :type Integer) (bFromSweep :type Boolean) (SweepResult :type Hit%20Result%20Structure%20%28by%20ref%29))
  (bind _asbp_player (Utilities|Casting|CastToBP_Player OtherActor))
  (Variables|/Game/Blueprints/BP_Player.BP_Player_C|SetCurrentInteractText _asbp_player "Locked"))

(event OnComponentEndOverlap(Trigger)
  (params (OverlappedComponent :type Primitive%20Component%20Object%20Reference) (OtherActor :type Actor%20Object%20Reference) (OtherComp :type Primitive%20Component%20Object%20Reference) (OtherBodyIndex :type Integer))
  (bind _asbp_player (Utilities|Casting|CastToBP_Player OtherActor))
  (Variables|/Game/Blueprints/BP_Player.BP_Player_C|SetCurrentInteractText _asbp_player ""))

(event EventBeginPlay
  (bind _returnvalue (Actor|GetActorOfClass "/Game/Blueprints/KeyScript.KeyScript_C"))
  (Variables|Default|SetWorldKey _returnvalue))

(event Collision|EventActorBeginOverlap
  (params (OtherActor :type Actor%20Object%20Reference)))

(event EventTick
  (params (DeltaSeconds :type Float%20%28single-precision%29))
  (if (Variables|/Game/Blueprints/KeyScript.KeyScript_C|GetDoors%20Open (Variables|Default|GetWorldKey))
    (Actor|DestroyActor)))

(fn ConstructionScript)