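; WinCondition is a trigger-box actor that shows a victory message when BP_Player stands still inside it for five seconds.
; Box overlap events toggle the Praying flag and set or clear the player's interact text.
; Tick compares the player's transform to last frame's, counting down while it is unchanged and resetting on any change or outside the box.
; Winning only changes the text and is not latched.
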(event OnComponentBeginOverlap(TriggerBox)
  (params (OverlappedComponent :type Primitive%20Component%20Object%20Reference) (OtherActor :type Actor%20Object%20Reference) (OtherComp :type Primitive%20Component%20Object%20Reference) (OtherBodyIndex :type Integer) (bFromSweep :type Boolean) (SweepResult :type Hit%20Result%20Structure%20%28by%20ref%29))
  (bind _asbp_player (Utilities|Casting|CastToBP_Player OtherActor))
  (Variables|/Game/Blueprints/BP_Player.BP_Player_C|SetCurrentInteractText _asbp_player "Be at peace")
  (Variables|Default|SetPraying true))

(event OnComponentEndOverlap(TriggerBox)
  (params (OverlappedComponent :type Primitive%20Component%20Object%20Reference) (OtherActor :type Actor%20Object%20Reference) (OtherComp :type Primitive%20Component%20Object%20Reference) (OtherBodyIndex :type Integer))
  (bind _asbp_player (Utilities|Casting|CastToBP_Player OtherActor))
  (Variables|/Game/Blueprints/BP_Player.BP_Player_C|SetCurrentInteractText _asbp_player "")
  (Variables|Default|SetPraying false))

(event EventBeginPlay
  (bind _returnvalue (Actor|GetActorOfClass "/Game/Blueprints/BP_Player.BP_Player_C"))
  (Variables|Default|SetPlayer _returnvalue)
  (Variables|Default|SetTimer 5.0))

(event Collision|EventActorBeginOverlap
  (params (OtherActor :type Actor%20Object%20Reference)))

(event EventTick
  (params (DeltaSeconds :type Float%20%28single-precision%29))
  (bind _player (Variables|Default|GetPlayer))
  (bind _returnvalue (Transformation|GetActorTransform _player))
  (if (Variables|Default|GetPraying)
    (Variables|/Game/Blueprints/BP_Player.BP_Player_C|SetCurrentInteractText _player "Be at peace (Stand still)")
    (if (== (Variables|Default|GetLastPos) _returnvalue)
      (Variables|Default|SetTimer (- (Variables|Default|GetTimer) DeltaSeconds))
      (else
        (Variables|Default|SetTimer 5.0 :!label _label)))
    (else
      (goto _label)))
  (Variables|Default|SetLastPos _returnvalue)
  (if (< (Variables|Default|GetTimer) 0.0)
    (Variables|/Game/Blueprints/BP_Player.BP_Player_C|SetCurrentInteractText _player "You did it :]")))

(fn ConstructionScript)